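; BP_AmbienceBox is a placeable volume that switches the level's ambience when the first-person player enters it.
; On BeginPlay it finds and stores the first BP_AmbienceController in the level.
; On overlap, a collapsed graph casts the other actor to BP_FirstPersonCharacter, then the controller's ChangeAmbience receives the box's AmbienceType.
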(event `self.ReceiveBeginPlay`
  ;[1 1 1] Get the Ambience Controller on Begin Play
  (bind _outactors (`GameplayStatics.GetAllActorsOfClass` "/Game/Blueprints/BP_AmbienceController.BP_AmbienceController_C"))
  (set `self.Ambience Controller` (`|GetArrayItem` _outactors)))

(event `self.ReceiveActorBeginOverlap`
  (params (OtherActor :type "Actor Object Reference"))
  (cast `/Game/FirstPerson/Blueprints/BP_FirstPersonCharacter` OtherActor)
  (if true
    (`/Game/Blueprints/BP_AmbienceController.ChangeAmbience` (`self.Ambience Controller`) (`self.Ambience Type`)) ; Change the ambience
  ))

(fn `UserConstructionScript`)