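; BP_LayerBox is an overlap trigger that changes a layer of the game's music when the first-person player character enters it.
; On BeginPlay it caches the first BP_MusicController found in the level.
; On a player overlap it passes its Layer and Playing state to the controller's ChangeLayer and stores the result back in Playing for the next overlap.
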(event `self.ReceiveBeginPlay`
  ;[1 1 1] Get the Music Controller on Begin Play
  (bind _outactors (`GameplayStatics.GetAllActorsOfClass` "/Game/Blueprints/BP_MusicController.BP_MusicController_C"))
  (set `self.Music Controller` (`|GetArrayItem` _outactors)))

(event `self.ReceiveActorBeginOverlap`
  (params (OtherActor :type "Actor Object Reference"))
  ;[1 1 1] Change the layer of the music on the overlap
  (cast `/Game/FirstPerson/Blueprints/BP_FirstPersonCharacter` OtherActor)
  (if true
    (bind _playing (`/Game/Blueprints/BP_MusicController.ChangeLayer` (`self.Music Controller`) (`self.Layer`) (`self.Playing`)))
    (set `self.Playing` _playing)))

(fn `UserConstructionScript`)