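; Music controller Blueprint that drives adaptive game music through two MetaSound audio components created on BeginPlay, one for horizontal sequencing and one for vertical layering.
; ChangeSequence sets a section index and fires triggers for Explore, Combat and Suspense, plus Start and Stop.
; ChangeLayer toggles four piano layers by trigger, returning the new playing state, and starts or stops them all.
; ChangeMusicVolume updates both components; ChangeAmbienceVolume is empty.
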(event `self.ReceiveBeginPlay`
  ;[1 1 1] Create and set the Horizontal Sequencing Audio Component
  (bind _returnvalue (`AddComponent|NODE_AddAudioComponent-0`))
  (set `self.HorizontalComponent` _returnvalue)
  ;[1 1 1] Create and set the Vertical Layering Audio Component
  (bind _returnvalue_2 (`AddComponent|NODE_AddAudioComponent-1`))
  (set `self.VerticalComponent` _returnvalue_2))

(fn `ChangeAmbienceVolume`)

(fn `ChangeLayer`
  (params (Layer :type "/Game/Blueprints/E_VerticalLayer Enum" :default "NewEnumerator0") (Play :type Boolean))
  (returns (Playing :type Boolean))
  (bind _verticalcomponent (`self.VerticalComponent`))
  (bind _verticalcomponent_2 (`self.VerticalComponent`))
  (bind _verticalcomponent_3 (`self.VerticalComponent`))
  (bind _verticalcomponent_4 (`self.VerticalComponent`))
  (switch `/Game/Blueprints/E_VerticalLayer` Layer
    (:`NewEnumerator0`
      ;[1 1 1] Toggle Layer One
      (if Play
        (`AudioParameterControllerInterface.SetTriggerParameter` _verticalcomponent_2 "On Stop P1")
        (return false)
        (else
          (`AudioParameterControllerInterface.SetTriggerParameter` _verticalcomponent_2 "On P1")
          (return true))))
    (:`NewEnumerator1`
      ;[1 1 1] Toggle Layer Two
      (if Play
        (`AudioParameterControllerInterface.SetTriggerParameter` _verticalcomponent_3 "On Stop P2")
        (return false)
        (else
          (`AudioParameterControllerInterface.SetTriggerParameter` _verticalcomponent_3 "On P2")
          (return true))))
    (:`NewEnumerator2`
      ;[1 1 1] Toggle Layer Three
      (if Play
        (`AudioParameterControllerInterface.SetTriggerParameter` _verticalcomponent_4 "On Stop P3")
        (return false)
        (else
          (`AudioParameterControllerInterface.SetTriggerParameter` _verticalcomponent_4 "On P3")
          (return true))))
    (:`NewEnumerator3`
      ;[1 1 1] Toggle Layer Four
      (if Play
        (`AudioParameterControllerInterface.SetTriggerParameter` _verticalcomponent "On Stop P4")
        (return false)
        (else
          (`AudioParameterControllerInterface.SetTriggerParameter` _verticalcomponent "On P4")
          (return true))))
    (:`NewEnumerator4`
      ;[1 1 1] Execute the Start trigger and set playing layer two by default
      (`AudioParameterControllerInterface.SetTriggerParameter` (`self.VerticalComponent`) "On Start")
      (return true))
    (:`NewEnumerator5`
      ;[1 1 1] Execute the Stop All trigger and set not playing any layers
      (`AudioParameterControllerInterface.SetTriggerParameter` (`self.VerticalComponent`) "On Stop All")
      (return false))))

(fn `ChangeMusicVolume`
  (params (Volume :type "Float (double-precision)"))
  ;[1 1 1] Set the volume in the MetaSound
  (`AudioParameterControllerInterface.SetFloatParameter` (`self.HorizontalComponent`) "Music Volume" Volume)
  (`AudioParameterControllerInterface.SetFloatParameter` (`self.VerticalComponent`) "Music Volume" Volume)
  (set `self.Volume` Volume))

(fn `ChangeSequence`
  (params (Section :type "/Game/Blueprints/E_HorizontalSection Enum" :default "NewEnumerator0"))
  (locals (Index :type Integer))
  (switch `/Game/Blueprints/E_HorizontalSection` Section
    (:`NewEnumerator0`
      ;[1 1 1] Set section
      (bind _output_get (set `local.Index` 1))
      (`AudioParameterControllerInterface.SetIntParameter` (`self.HorizontalComponent`) "Section Index" _output_get)
      (`AudioParameterControllerInterface.SetTriggerParameter` (`self.HorizontalComponent`) "On Explore"))
    (:`NewEnumerator1`
      (bind _output_get_2 (set `local.Index` 3))
      (`AudioParameterControllerInterface.SetIntParameter` (`self.HorizontalComponent`) "Section Index" _output_get_2)
      (`AudioParameterControllerInterface.SetTriggerParameter` (`self.HorizontalComponent`) "On Combat"))
    (:`NewEnumerator2`
      (bind _output_get_3 (set `local.Index` 2))
      (`AudioParameterControllerInterface.SetIntParameter` (`self.HorizontalComponent`) "Section Index" _output_get_3)
      (`AudioParameterControllerInterface.SetTriggerParameter` (`self.HorizontalComponent`) "On Suspense"))
    (:`NewEnumerator3`
      ;[1 1 1] Stop the music
      (`AudioParameterControllerInterface.SetTriggerParameter` (`self.HorizontalComponent`) "On Stop"))
    (:`NewEnumerator4`
      ;[1 1 1] Start the music
      (`AudioParameterControllerInterface.SetTriggerParameter` (`self.HorizontalComponent`) "On Start"))))

(fn `UserConstructionScript`)